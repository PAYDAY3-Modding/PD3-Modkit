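; Placeable drone Blueprint that, when activated, spawns a BP_Moon_Gun at the local player pawn's transform.
; It overrides the spawned gun's team ID and hacked-by-player array, then sets the faction on its armed-pawn AI controller.
; The sensor ammo-depleted event, construction script and other events are empty.
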(event Custom|OnSensorAmmoDepleted_Event_0)

(event Collision|EventActorBeginOverlap
  (params (OtherActor :type Actor%20Object%20Reference)))

(event EventTick
  (params (DeltaSeconds :type Float%20%28single-precision%29)))

(event EventOnActivated
  (bind _returnvalue (Game|SpawnActorfromClass "/Game/DLCs/00005-DLCHEIST0001/Gameplay/AI/Moon/BP_Moon_Gun.BP_Moon_Gun_C" (Transformation|GetActorTransform (Class|SBZPlayerLibrary|GetLocalPlayerPawn)) "AdjustIfPossibleButAlwaysSpawn" "MultiplyWithRoot" 0 0))
  (Variables|/Script/Starbreeze.SBZAIDrone|SetTeamID _returnvalue (Utilities|Struct|MakeGenericTeamId 0))
  (Variables|/Script/Starbreeze.SBZAIDrone|SetHackedByPlayerArray _returnvalue (Utilities|Array|MakeArray (Utilities|Struct|MakeUniqueNetIdRepl)))
  (bind _assbzaiarmed_pawn_controller (Utilities|Casting|CastToSBZAIArmedPawnController (AI|GetAIController _returnvalue)))
  (Variables|/Script/Starbreeze.SBZAIArmedPawnController|SetFaction _assbzaiarmed_pawn_controller (Utilities|Struct|MakeSBZFactionIdHelper)))

(event EventBeginPlay)

(fn ConstructionScript)
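; A general-purpose Blueprint function library of small helpers for math, text and character queries.
; Float helpers cover absolute difference, near-zero testing, safe reciprocal and positive or negative infinity parsed from strings.
; String and text helpers trim both ends to detect empty or whitespace-only values.
; Character helpers expose alive state and gather all SBZCharacter actors matching a team ID, a lookup noted as untested.
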(fn Difference(float)
  (params (A :type Float%20%28double-precision%29) (B :type Float%20%28double-precision%29))
  (return (Math|Float|Absolute(Float) (- A B))))

(fn IsZero(float)
  (params (A :type Float%20%28double-precision%29))
  (return (Math|Float|NearlyEqual(Float) A 0.0 0.0001)))

(fn Invert(float)
  (params (A :type Float%20%28double-precision%29))
  (return (Math|Float|SafeDivide 1.0 A)))

(fn TextIsEmptyorWhitespace
  (params (InText :type Text%20%28by%20ref%29))
  (return (Utilities|Text|TextIsEmpty (Class|KismetTextLibrary|TextTrimPrecedingandTrailing InText))))

(fn Infinity(float)
  (return (Math|Conversions|ToFloat(Integer) "inf")))

(fn -Infinity(float)
  (return (Math|Conversions|ToFloat(Integer) "-inf")))

(fn GetAllCharactersOfTeam
  (params (Team :type ETeamAttitude%20Enum :default "Friendly"))
  (bind _outactors (Actor|GetAllActorsOfClass 0 "/Script/Starbreeze.SBZCharacter"))
  (for _array_element _outactors
    (if (== (Math|Byte|MakeLiteralByte Team) (.teamid (Variables|/Script/Starbreeze.SBZCharacter|GetTeamID _array_element)))
      (Utilities|Array|AddUnique (LocalVariables|GetCharacterArray) _array_element)))
  (return (LocalVariables|GetCharacterArray)))

(fn TrimPrecedingandTrailing
  (params (SourceString :type String))
  (return (Utilities|String|TrimTrailing (Utilities|String|Trim SourceString))))

(fn IsEmptyorWhitespace
  (params (SourceString :type String))
  (return (Utilities|Array|IsEmpty (Utilities|String|TrimPrecedingandTrailing SourceString))))

(fn IsAlive
  (params (Character :type SBZ%20Character%20Object%20Reference))
  (return (Variables|/Script/Starbreeze.SBZCharacter|GetbIsAlive Character)))